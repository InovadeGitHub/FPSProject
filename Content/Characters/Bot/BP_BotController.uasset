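; AI controller for bot characters that runs the BT_Bot behavior tree on possession and reports when it sees the player.
; AI Perception updates are filtered to BP_Player and the sight sense, then a Sight graph writes the sensed result to the bCanSeePlayer blackboard key.
; Small helper functions wrap Blackboard bool and object writes, though only the bool helper is used here.
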(event `self.ReceivePossess`
  (params (PossessedPawn :type "Pawn Object Reference"))
  (`self.RunBehaviorTree` "/Game/Characters/Bot/AI/BT_Bot.BT_Bot"))

(event `self.AIPerception.OnTargetPerceptionUpdated`
  (params (Actor :type "Actor Object Reference") (Stimulus :type "AIStimulus Structure"))
  (cast `/Game/Characters/Player/BP_Player` Actor)
  (bind _returnvalue (`AIPerceptionSystem.GetSenseClassForStimulus` Stimulus))
  (if (== _returnvalue "/Script/AIModule.AISense_Sight")
    (`self.Update Boolean Key` "bCanSeePlayer" (`.bSuccessfullySensed` (break `AIStimulus` Stimulus)))))

(fn `Update Boolean Key`
  (params (`Key Name` :type Name) (`Key Value` :type Boolean))
  (`BlackboardComponent.SetValueAsBool` (`AIBlueprintHelperLibrary.GetBlackboard` null) `Key Name` `Key Value`))

(fn `Update Object Key`
  (params (`Key Value` :type "Object Object Reference") (`Key Name` :type Name))
  (`BlackboardComponent.SetValueAsObject` (`AIBlueprintHelperLibrary.GetBlackboard` null) `Key Name` `Key Value`))

(fn `UserConstructionScript`)