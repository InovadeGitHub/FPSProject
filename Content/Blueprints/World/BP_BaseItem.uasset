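; BP_BaseItem is a base actor for world items that can be picked up and dropped.
; The construction script applies the mesh from ItemSettings to its StaticMesh.
; OnPickup makes the mesh ignore all collision and stops physics simulation.
; OnDrop detaches the actor in world space, then restores blocking collision and physics so it moves as a loose object.
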(event `/Game/GameplayLogic/BlueprintInterfaces/BPI_Pickable.On Pickup`
  (bind _staticmesh (`self.StaticMesh`))
  (`PrimitiveComponent.SetCollisionResponseToAllChannels` _staticmesh "ECR_Ignore")
  (`PrimitiveComponent.SetSimulatePhysics` _staticmesh false))

(event `/Game/GameplayLogic/BlueprintInterfaces/BPI_Pickable.On Drop`
  (bind _staticmesh (`self.StaticMesh`))
  (`self.K2_DetachFromActor` "KeepWorld" "KeepWorld" "KeepWorld")
  (`PrimitiveComponent.SetCollisionResponseToAllChannels` _staticmesh "ECR_Block")
  (`PrimitiveComponent.SetSimulatePhysics` _staticmesh true))

(fn `UserConstructionScript`
  (`StaticMeshComponent.SetStaticMesh` (`self.StaticMesh`) (`.ItemMesh_8_041E06DB40992BB9B25732BEF0E7FEC6` (break `/Game/Blueprints/Structures/STR_Item_Settings` (`self.Item Settings`)))))