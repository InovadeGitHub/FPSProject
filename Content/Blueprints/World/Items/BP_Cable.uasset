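; BP_Cable is an inventory item that the player plugs onto a surface they target.
; On apply, it runs a short, debug-drawn line trace from the player and stores any hit location as the plug point.
; It moves its mesh there with a look-at rotation toward that point, attaches it to the hit component keeping world transform, then removes itself from the player's inventory.
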(event `/Game/GameplayLogic/BlueprintInterfaces/BPI_Interactable.On Start Apply`
  (params (Player :type "/Game/Characters/Player/BP_Player Object Reference"))
  (bind _staticmesh (`self.StaticMesh`))
  (bind (_out_hit _returnvalue) (`/Game/Characters/Player/BP_Player.Linetrace` Player 250.0 true))
  (if _returnvalue
    (bind (_bblockinghit _binitialoverlap _time _distance _location _impactpoint _normal _impactnormal _physmat _hitactor _hitcomponent) (`GameplayStatics.BreakHitResult` _out_hit))
    (bind _output_get (set `self.Cable Plug Point` _location))
    (`SceneComponent.K2_SetWorldLocationAndRotation` _staticmesh _output_get (`KismetMathLibrary.FindLookAtRotation` (`SceneComponent.K2_GetComponentLocation` (`self.StaticMesh`)) _location) false false)
    (`SceneComponent.K2_AttachToComponent` _staticmesh _hitcomponent "None" "KeepWorld" "KeepWorld" "KeepWorld" true)
    (`/Game/Blueprints/Components/BP_InventoryComponent.Remove Item` (`/Game/Characters/BP_BaseCharacter.InventoryComponent` Player) self)))

(fn `UserConstructionScript`
  (`parent.UserConstructionScript`))