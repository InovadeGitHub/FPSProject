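; Actor component that stores an electric power level for its owner and reports changes through an OnPowerChanged event.
; AddPower and SubtractPower adjust the level, clamp it between empty and full, then broadcast the new value with a HasPower flag.
; HasPower is true only at exactly full charge, so partial power counts as unpowered.
; BeginPlay broadcasts the initial state.
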(event `self.ReceiveBeginPlay`
  ;[1 0.3002 0.8321] Begin Play
  (`self.On Power Changed` (`self.Has Power`) (`self.Power`)))

(fn `Add Power`
  (params (`Amount To Add` :type "Float (double-precision)"))
  (bind _output_get (set `self.Power` (`KismetMathLibrary.FClamp` (+ (`self.Power`) `Amount To Add`) 0.0 100.0)))
  (`self.On Power Changed` (`self.Has Power`) _output_get))

(fn `Has Power`
  (returns (ReturnValue :type Boolean))
  (return (== (`self.Power`) 100.0)))

(fn `Subtract Power`
  (params (`Amount To Subtract` :type "Float (double-precision)"))
  (bind _output_get (set `self.Power` (`KismetMathLibrary.FClamp` (- (`self.Power`) `Amount To Subtract`) 0.0 100.0)))
  (`self.On Power Changed` (`self.Has Power`) _output_get))