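; Inventory component that adds and removes items in an ItemInventory collection, capped at MaximumInventoryCapacity.
; AddItem checks that the inventory is not full, then stores the Add result in SelectedItem.
; RemoveItem requires the item to be present and HasItem to pass, though that count >= 0 check is always true.
; Successful changes print a colored on-screen message built from an Added/Removed enum.
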(fn `Add Item`
  (params (`Item To Add` :type "/Game/Blueprints/World/BP_BaseItem Object Reference (by ref)"))
  (returns (ReturnValue :type Boolean))
  (bind _returnvalue (not (`self.Is Inventory Full`)))
  (if _returnvalue
    (bind _returnvalue_2 (`KismetArrayLibrary.Array_Add` (`self.Item Inventory`) `Item To Add`))
    (set `self.Selected Item` _returnvalue_2)
    (`self.Print Strings` "NewEnumerator0")
    (return _returnvalue)))

(fn `Has Item`
  (returns (ReturnValue :type Boolean))
  (return (>= (`self.Return Items`) 0)))

(fn `Is Inventory Full`
  (returns (ReturnValue :type Boolean))
  (return (== (`self.Return Items`) (`self.Maximum Inventory Capacity`))))

(fn `Print Strings`
  (params (Type :type "/Game/Blueprints/Enumerations/Debug/ENUM_Debug_InventoryType Enum" :default "NewEnumerator0"))
  (`KismetSystemLibrary.PrintString` (`KismetStringLibrary.Concat_StrStr` "Item Has Been " (`|GetEnumeratorNameAsString` Type) (select `/Game/Blueprints/Enumerations/Debug/ENUM_Debug_InventoryType` Type :`NewEnumerator0` " To " :`NewEnumerator1` " From ") "Inventory.") true true (struct :`R` 1.0 :`G` 0.564963 :`B` 0.203346 :`A` 1.0) 1.0))

(fn `Remove Item`
  (params (`Item To Remove` :type "/Game/Blueprints/World/BP_BaseItem Object Reference"))
  (if (and (`KismetArrayLibrary.Array_Contains` (`self.Item Inventory`) `Item To Remove`) (`self.Has Item`))
    (bind _returnvalue (`KismetArrayLibrary.Array_RemoveItem` (`self.Item Inventory`) `Item To Remove`))
    (if _returnvalue
      (`self.Print Strings` "NewEnumerator1"))))

(fn `Return Items`
  (returns (ReturnValue :type Integer))
  (return (`KismetArrayLibrary.Array_Length` (`self.Item Inventory`))))